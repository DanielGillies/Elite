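; BP_GoalPost is a capture objective that reports victory once attackers have occupied its TriggerArea for the capture time.
; An AttackerCharacter entering sets an overlap flag, which lets Tick accumulate and print elapsed time, then print VICTORY.
; On exit, the flag clears only if other attackers still overlap, so a last attacker leaving keeps the timer running.
; Elapsed time never resets, and victory is only a printed message.
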(event `self.ReceiveTick`
  (params (DeltaSeconds :type "Float (single-precision)"))
  (if (`self.IsOverlapping`)
    (if (< (`self.ElapsedTime`) (`self.CaptureTime`))
      (bind _output_get (set `self.ElapsedTime` (+ (`self.ElapsedTime`) DeltaSeconds)))
      (`KismetSystemLibrary.PrintString` (`KismetStringLibrary.Conv_DoubleToString` _output_get))
      (else
        (`KismetSystemLibrary.PrintString` "VICTORY")))))

(event `self.TriggerArea.OnComponentBeginOverlap`
  (params (OverlappedComponent :type "PrimitiveComponent Object Reference") (OtherActor :type "Actor Object Reference") (OtherComp :type "PrimitiveComponent Object Reference") (OtherBodyIndex :type Integer) (bFromSweep :type Boolean) (SweepResult :type "HitResult Structure (by ref)"))
  (cast `AttackerCharacter` OtherActor)
  (if true
    (set `self.IsOverlapping` true)))

(event `self.TriggerArea.OnComponentEndOverlap`
  (params (OverlappedComponent :type "PrimitiveComponent Object Reference") (OtherActor :type "Actor Object Reference") (OtherComp :type "PrimitiveComponent Object Reference") (OtherBodyIndex :type Integer))
  (cast `AttackerCharacter` OtherActor)
  (if true
    (if (> (`KismetArrayLibrary.Array_Length` (`PrimitiveComponent.GetOverlappingActors` (`self.TriggerArea`) "/Script/Elite.AttackerCharacter")) 0)
      (set `self.IsOverlapping` false))))

(fn `UserConstructionScript`)