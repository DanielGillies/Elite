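; Attacker character Blueprint that fires a cosmetic hitscan beam when the Fire action is pressed.
; A Visibility line trace runs forward from player 0's camera, and a P_Beam emitter stretches from just below the camera to the hit point or maximum range.
; A blocking hit also spawns a P_Explosion with auto-destroy off; the graph applies no damage.
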(event `InputAction|Fire`
  (params (Key :type "Key Structure" :default "AnyKey"))
  (bind _returnvalue (`GameplayStatics.GetPlayerCameraManager` 0))
  (bind _returnvalue_2 (`self.K2_GetActorLocation` _returnvalue))
  (bind _returnvalue_3 (+ (* (`SceneComponent.GetForwardVector` (`PlayerCameraManager.TransformComponent` _returnvalue)) 5000.0) _returnvalue_2))
  (:`Pressed`
    (bind _outhit (`KismetSystemLibrary.LineTraceSingle` _returnvalue_2 _returnvalue_3 "TraceTypeQuery1"))
    (bind (_bblockinghit _binitialoverlap _time _location) (`GameplayStatics.BreakHitResult` _outhit))
    (if _bblockinghit
      (bind _returnvalue_4 (`GameplayStatics.SpawnEmitterAtLocation` "/Game/Particles/P_Beam.P_Beam" _returnvalue_2))
      (`ParticleSystemComponent.SetBeamSourcePoint` _returnvalue_4 0 (- _returnvalue_2 (0.0 0.0 20.0)) 0)
      (`ParticleSystemComponent.SetBeamTargetPoint` _returnvalue_4 0 _location 0)
      (`GameplayStatics.SpawnEmitterAtLocation` "/Game/StarterContent/Particles/P_Explosion.P_Explosion" _location (struct) false)
      (else
        (bind _returnvalue_5 (`GameplayStatics.SpawnEmitterAtLocation` "/Game/Particles/P_Beam.P_Beam" _returnvalue_2))
        (`ParticleSystemComponent.SetBeamSourcePoint` _returnvalue_5 0 (- _returnvalue_2 (0.0 0.0 20.0)) 0)
        (`ParticleSystemComponent.SetBeamTargetPoint` _returnvalue_5 0 _returnvalue_3 0)))))

(fn `UserConstructionScript`)